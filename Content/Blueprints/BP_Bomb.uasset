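; Grid-based bomb that detonates after a timed delay, spawning explosion actors on its own tile and along set directions up to its range.
; Each direction gets one line trace, and a blocking hit shortens the blast to the whole tiles before it, computed from range times hit time.
; After spawning the explosions, it returns one bomb ammo to the owning player and destroys itself.
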(event `self.ReceiveBeginPlay`
  (`KismetSystemLibrary.Delay` (`self.DetonationTime`))
  (`self.Explode`))

(event `Explode`
  ;[1 1 1] quick and functional code, should be optimized (stat scenegraph shows no bumps in performance, but still it's many raycasts and actor spawns in a nested for loop)
  (for _array_element (`self.LinetraceDirections`)
    (bind _explodingtilespots (`self.LinetraceBombExplosion` _array_element))
    (for _array_element_2 _explodingtilespots
      (`|SpawnActorFromClass` "/Game/Blueprints/BP_Explosion.BP_Explosion_C" (`KismetMathLibrary.MakeTransform` (+ _array_element_2 (`self.K2_GetActorLocation`))) "AlwaysSpawn" "OverrideRootScale" null null)))
  (`|SpawnActorFromClass` "/Game/Blueprints/BP_Explosion.BP_Explosion_C" (`KismetMathLibrary.MakeTransform` (`self.K2_GetActorLocation`)) "AlwaysSpawn" "OverrideRootScale" null null) ; explosion on bomb location, requires no check
  (`/Engine/EditorBlueprintResources/StandardMacros.IncrementInt` (`/Game/Blueprints/BP_BomberCharacter.CurrentBombAmmo` (`self.OwningPlayer`))
    (:`  `
      (`self.K2_DestroyActor`))))

(fn `GetNumTilesHit`
  (params (Hit :type "HitResult Structure (by ref)"))
  (returns (ReturnValue :type Integer))
  (return (`KismetMathLibrary.FFloor` (* (`self.Range`) (`.Time` (`GameplayStatics.BreakHitResult` Hit))))))

(fn `LinetraceBombExplosion`
  (params (Direction :type "Vector Structure"))
  (returns (ExplodingTileSpots :type "Array of Vector Structure"))
  (locals (VerifiedTiles :type "Array of Vector Structure") (MyDirection :type "Vector Structure"))
  (bind _returnvalue (`self.K2_GetActorLocation`))
  (set `local.MyDirection` Direction)
  (bind (_outhit _returnvalue_2) (`KismetSystemLibrary.LineTraceSingle` _returnvalue (+ (* (`local.MyDirection`) (* (`self.Range`) 50)) _returnvalue) "TraceTypeQuery1")) ; make a line trace check {range} tiles towards the direction (this function is called once per direction)
  (if _returnvalue_2
    (bind _returnvalue_3 (`self.GetNumTilesHit` _outhit))
    (if (> _returnvalue_3 0)
      (for _index (range 1 (+ _returnvalue_3 1))
        (`KismetArrayLibrary.Array_Add` (`local.VerifiedTiles`) (* (`local.MyDirection`) (* _index 50))))
      (return (`local.VerifiedTiles`))
      (else
        (return (`local.VerifiedTiles`))))
    (else
      (for _index_2 (range 1 (+ (`self.Range`) 1))
        (`KismetArrayLibrary.Array_Add` (`local.VerifiedTiles`) (* (`local.MyDirection`) (* _index_2 50))))
      (return (`local.VerifiedTiles`)))))

(fn `UserConstructionScript`)