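; Player character for a Bomberman-style game that drops bombs snapped to a grid.
; On BeginPlay it spawns and possesses its own PlayerController as a quick local two-player workaround.
; SpawnBomb checks ammo through HasBombs, rounds its location via ConstrainPointToGrid, and spawns a BP_Bomb carrying its detonation time, range and owner.
; A successful spawn decrements ammo, which the bomb is expected to restore when it explodes.
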(event `self.ReceiveBeginPlay`
  ;[1 1 1] Pawns need a controller to accept input. This is part of the quick and dirty solution for 2-player multiplay
  (bind _returnvalue (`|SpawnActorFromClass` "/Script/Engine.PlayerController" (`KismetMathLibrary.MakeTransform` (0.0 0.0 0.0)) "AlwaysSpawn" "OverrideRootScale" null null))
  (`Controller.Possess` _returnvalue self))

(event `SpawnBomb`
  (bind (_returnvalue_x _returnvalue_y) (`KismetMathLibrary.BreakVector` (`self.K2_GetActorLocation`)))
  ;[1 0.154 0.294] Spawning bombs!
  (`self.HasBombs`
    (:`true`
      (bind _returnvalue (`|SpawnActorFromClass` "/Game/Blueprints/BP_Bomb.BP_Bomb_C" (`KismetMathLibrary.MakeTransform` (`KismetMathLibrary.MakeVector` (`KismetMathLibrary.Conv_IntToDouble` (`self.ConstrainPointToGrid` _returnvalue_x 50)) (`KismetMathLibrary.Conv_IntToDouble` (`self.ConstrainPointToGrid` _returnvalue_y 50)) 50.0)) "AlwaysSpawn" "OverrideRootScale" null (`self.BombDetonationTime`) (`self.BombRange`) self null))
      (`/Engine/EditorBlueprintResources/StandardMacros.IsValid` _returnvalue ; check if we were not able to spawn the bomb for whatever reason
        (:`Is Valid`
          (`/Engine/EditorBlueprintResources/StandardMacros.DecrementInt` (`self.CurrentBombAmmo`)) ; the bomb will get back at the player when it explodes and increment his bomb count
        )))))

(fn `ConstrainPointToGrid`
  (params (Float :type "Float (double-precision)") (GridSize :type Integer))
  (returns (ReturnValue :type Integer))
  ;[1 1 1] This function is used to spawn bombs and the like in accurate positions
  (return (* (`KismetMathLibrary.Round` (/ Float (`KismetMathLibrary.Conv_IntToDouble` GridSize))) GridSize)))

(fn `UserConstructionScript`)