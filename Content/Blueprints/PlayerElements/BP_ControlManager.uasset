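; BP_ControlManager is the central input and UI hub for two players in a bomber-style game.
; On BeginPlay it creates the single shared game interface widget, then gives both player references their index and that widget.
; It routes separate per-player input axes and actions straight to each player as world X/Y movement and bomb spawning, so one Blueprint drives both characters.
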(event `self.ReceiveBeginPlay`
  ;[0.8617 1 0] Setup player index and UI - there is only one UI widget in this game
  (bind _returnvalue (`|CreateWidget` "/Game/Blueprints/UserInterface/UI_BomberGameInterface.UI_BomberGameInterface_C"))
  (set `self.UI` _returnvalue)
  (`UserWidget.AddToPlayerScreen` _returnvalue 0)
  (set `/Game/Blueprints/PlayerElements/BP_BomberCharacter.PlayerIndex` 0 (`self.Player1`))
  (set `/Game/Blueprints/PlayerElements/BP_BomberCharacter.PlayerIndex` 1 (`self.Player2`))
  (set `/Game/Blueprints/PlayerElements/BP_BomberCharacter.UI` (`self.UI`) (`self.Player1`))
  (set `/Game/Blueprints/PlayerElements/BP_BomberCharacter.UI` (`self.UI`) (`self.Player2`)))

(event `InputAxis|MoveUp1` :consume false
  (params (AxisValue :type "Float (single-precision)"))
  ;[1 1 1] Movement First Player
  (`self.AddMovementInput` (`self.Player1`) (`KismetMathLibrary.MakeVector` 0.0 AxisValue) 1.0 false))

(event `InputAxis|MoveUp2` :consume false
  (params (AxisValue :type "Float (single-precision)"))
  ;[1 1 1] Movement second player
  (`self.AddMovementInput` (`self.Player2`) (`KismetMathLibrary.MakeVector` 0.0 AxisValue) 1.0 false))

(event `InputAxis|MoveRight1` :consume false
  (params (AxisValue :type "Float (single-precision)"))
  ;[1 1 1] Movement First Player
  (`self.AddMovementInput` (`self.Player1`) (`KismetMathLibrary.MakeVector` AxisValue) 1.0 false))

(event `InputAxis|MoveRight2` :consume false
  (params (AxisValue :type "Float (single-precision)"))
  ;[1 1 1] Movement second player
  (`self.AddMovementInput` (`self.Player2`) (`KismetMathLibrary.MakeVector` AxisValue) 1.0 false))

(event `InputAction|SpawnBomb1`
  (params (Key :type "Key Structure"))
  ;[1 1 1] Placing Bombs
  (:`Pressed`
    (`/Game/Blueprints/PlayerElements/BP_BomberCharacter.SpawnBomb` (`self.Player1`))))

(event `InputAction|SpawnBomb2`
  (params (Key :type "Key Structure"))
  ;[1 1 1] Placing Bombs
  (:`Pressed`
    (`/Game/Blueprints/PlayerElements/BP_BomberCharacter.SpawnBomb` (`self.Player2`))))

(fn `UserConstructionScript`)