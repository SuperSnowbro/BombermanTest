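; BP_BomberCharacter is the player character for a two-player bomber game, spawning and possessing its own PlayerController on BeginPlay.
; Bomb requests go to a swappable spawner component, with timed-bomb pickups temporarily replacing the regular one through a retriggerable delay.
; Pickups raise range, ammo or walk speed, with UI updates for bomb stats.
; Death teleports the character away and notifies the game instance; random-point respawn with retry exists but is unused.
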(event `self.ReceiveBeginPlay`
  ;[1 1 1] Pawns need a controller to accept input. This is part of the quick and dirty solution for 2-player multiplay
  (bind _returnvalue (`|SpawnActorFromClass` "/Script/Engine.PlayerController" (`KismetMathLibrary.MakeTransform` (0.0 0.0 0.0)) "AlwaysSpawn" "OverrideRootScale" null null))
  (set `self.MyController` _returnvalue)
  (`Controller.Possess` _returnvalue self)
  ;[0 1 0.1986] Setup bomb spawner swapping system
  (set `self.CurrentBombSpawner` (`self.BPC_BombSpawn_Regular`))
  (set `/Game/Blueprints/PlayerElements/BPC_BombSpawnerComponent.MyOwnerCharacter` self (`self.BPC_BombSpawn_Timed`))
  (set `/Game/Blueprints/PlayerElements/BPC_BombSpawnerComponent.MyOwnerCharacter` self (`self.BPC_BombSpawn_Regular`))
  ;[1 1 1] Quick and dirty solution to death and respawn - setup
  (bind _outactors (`GameplayStatics.GetAllActorsOfClass` "/Game/Blueprints/LevelElements/BP_RespawnPoint.BP_RespawnPoint_C"))
  (set `self.RespawnPoints` _outactors))

(event `Die`
  (`self.K2_SetActorLocation` (`self.MyDeathLocation`) false true)
  (set `self.IsDead` true)
  (bind _asbp_bomber_game_instance (cast `/Game/Blueprints/BP_BomberGameInstance` (`GameplayStatics.GetGameInstance`)))
  (`/Game/Blueprints/BP_BomberGameInstance.PlayerDied` _asbp_bomber_game_instance (`self.PlayerIndex`)))

(event `SpawnBomb`
  ;[1 0.154 0.294] Spawning bombs!
  (if (not (`self.IsDead`))
    (`/Game/Blueprints/PlayerElements/BPC_BombSpawnerComponent.RequestBombSpawn` (`self.CurrentBombSpawner`))))

(event `AttemptRespawn`
  ;[1 1 1] Quick and dirty solution to death and respawn - not used - just plug the Die event in SetActorLocation to make this a reality!
  (bind _success (`self.Respawn`))
  (if (not _success)
    (`KismetSystemLibrary.PrintString` "Respawn unsuccessful, attempting again" false true (struct :`G` 0.66 :`B` 1.0 :`A` 1.0) 1.0) ; we print something so that we can see it in the log to easily spot infinite loops due to #badleveldesign
    (`KismetSystemLibrary.Delay` 0.05) ; we don't want to risk crashing from an infinite loop because of a problem with spawn points
    (`self.AttemptRespawn`)))

(event `CollectBombPowerPickup`
  ;[1 1 1] "easy" pickups!
  (`/Engine/EditorBlueprintResources/StandardMacros.IncrementInt` (`self.BombRange`) ; it will not affect previously placed bombs.
    (:`  `
      (`/Game/Blueprints/UserInterface/UI_BomberGameInterface.UpdateBombRange` (`self.UI`) (`self.PlayerIndex`) (`self.BombRange`)))))

(event `UpdateBombAmmoUI`
  (`/Game/Blueprints/UserInterface/UI_BomberGameInterface.UpdateBombs` (`self.UI`) (`self.PlayerIndex`) (`self.CurrentBombAmmo`)))

(event `CollectBombAmmo`
  ;[1 1 1] "easy" pickups!
  (`/Engine/EditorBlueprintResources/StandardMacros.IncrementInt` (`self.CurrentBombAmmo`)
    (:`  `
      (`self.UpdateBombAmmoUI`))))

(event `CollectSpeedPickup`
  (bind _charactermovement (`self.CharacterMovement`))
  ;[1 1 1] "easy" pickups!
  (set `CharacterMovementComponent.MaxWalkSpeed` (+ (`CharacterMovementComponent.MaxWalkSpeed` _charactermovement) (`self.PickupSpeedIncrement`)) _charactermovement))

(event `CollectTimeBombPickup`
  ;[1 1 1] Pickups that alter bomb type!
  (`/Game/Blueprints/UserInterface/UI_BomberGameInterface.TimeBombPickup` (`self.UI`) (`self.PlayerIndex`) (`self.TimeBombPickupDuration`))
  (`|ExecutionSequence`
    (:`then_0`
      (if (!= (`self.CurrentBombSpawner`) (`self.BPC_BombSpawn_Timed`))
        (`/Game/Blueprints/PlayerElements/BPC_BombSpawnerComponent.Dismiss` (`self.CurrentBombSpawner`)) ; if we collect a time bomb pickup, we let the previous bomb spawner know he has been replaced; unless it's a time bomb!  Useful only when multiple bomb spawn methods are used
      ))
    (:`then_1`
      (set `self.CurrentBombSpawner` (`self.BPC_BombSpawn_Timed`))
      (`self.CallResetBombSpawner` (`self.TimeBombPickupDuration`)))))

(event `CallResetBombSpawner`
  (params (Delay :type "Float (double-precision)"))
  ;[1 1 1] Pickups that alter bomb type!
  (`KismetSystemLibrary.RetriggerableDelay` Delay)
  (`self.ResetBombSpawner`))

(event `ResetBombSpawner`
  ;[1 1 1] Pickups that alter bomb type!
  (`/Game/Blueprints/PlayerElements/BPC_BombSpawnerComponent.Dismiss` (`self.CurrentBombSpawner`)) ; if we collect a time bomb pickup, we let the previous bomb spawner know he has been replaced; unless it's a time bomb!  Useful only when multiple bomb spawn methods are used
  (set `self.CurrentBombSpawner` (`self.BPC_BombSpawn_Regular`)))

(fn `ChangeAmmo`
  (params (AmmoChange :type Integer))
  (set `self.CurrentBombAmmo` (+ (`self.CurrentBombAmmo`) AmmoChange))
  (`self.UpdateBombAmmoUI`))

(fn `Respawn`
  (returns (success :type Boolean))
  (locals (PickedSpawnPoint :type "/Game/Blueprints/LevelElements/BP_RespawnPoint Object Reference"))
  (bind _respawnpoints (`self.RespawnPoints`))
  (bind _output_get (set `local.PickedSpawnPoint` (`|GetArrayItem` _respawnpoints (`KismetMathLibrary.RandomInteger` (`KismetArrayLibrary.Array_Length` _respawnpoints))))) ; we pick a random spawn point
  (bind _isavailable (`/Game/Blueprints/LevelElements/BP_RespawnPoint.IsAvailable` _output_get)) ; if point has no players nearby, it is available.
  (if _isavailable
    (`self.K2_SetActorLocation` (`self.K2_GetActorLocation` (`local.PickedSpawnPoint`)) false true)
    (set `self.IsDead` false)
    (return true)
    (else
      (return false))))

(fn `UserConstructionScript`)