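; BP_DestructibleWall is a level wall that bombs can destroy, with a chance to leave a pickup behind.
; BombRaycastHit rolls against PickupSpawnChance and may call SpawnPickup, then calls Die to destroy the actor and returns true.
; SpawnPickup spawns a random class from PickupClasses at the wall's location, always spawning regardless of collision.
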(event `Die`
  (`self.K2_DestroyActor`))

(fn `BombRaycastHit`
  (returns (HasBeenHit :type Boolean))
  (`|ExecutionSequence`
    (:`then_0`
      (if (not (> (`KismetMathLibrary.RandomFloat`) (`self.PickupSpawnChance`)))
        (`self.SpawnPickup`)))
    (:`then_1`
      (`self.Die`)
      (return true))))

(fn `SpawnPickup`
  (bind _pickupclasses (`self.PickupClasses`))
  (`|SpawnActorFromClass` (`|GetArrayItem` _pickupclasses (`KismetMathLibrary.RandomInteger` (`KismetArrayLibrary.Array_Length` _pickupclasses))) (`KismetMathLibrary.MakeTransform` (`self.K2_GetActorLocation`)) "AlwaysSpawn" "OverrideRootScale" null null))

(fn `UserConstructionScript`)