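; BP_ControlManager routes local input for two players, covering movement and bomb spawning.
; Each player has separate axis mappings that feed AddMovementInput on the Player1 or Player2 reference, with up on world Y and right on world X.
; Each player's SpawnBomb action press calls SpawnBomb on that player, so one Blueprint drives both characters.
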(event `InputAxis|MoveUp1` :consume false
  (params (AxisValue :type "Float (single-precision)"))
  ;[1 1 1] Movement First Player
  (`self.AddMovementInput` (`self.Player1`) (`KismetMathLibrary.MakeVector` 0.0 AxisValue) 1.0 false))

(event `InputAxis|MoveUp2` :consume false
  (params (AxisValue :type "Float (single-precision)"))
  ;[1 1 1] Movement second player
  (`self.AddMovementInput` (`self.Player2`) (`KismetMathLibrary.MakeVector` 0.0 AxisValue) 1.0 false))

(event `InputAxis|MoveRight1` :consume false
  (params (AxisValue :type "Float (single-precision)"))
  ;[1 1 1] Movement First Player
  (`self.AddMovementInput` (`self.Player1`) (`KismetMathLibrary.MakeVector` AxisValue) 1.0 false))

(event `InputAxis|MoveRight2` :consume false
  (params (AxisValue :type "Float (single-precision)"))
  ;[1 1 1] Movement second player
  (`self.AddMovementInput` (`self.Player2`) (`KismetMathLibrary.MakeVector` AxisValue) 1.0 false))

(event `InputAction|SpawnBomb1`
  (params (Key :type "Key Structure"))
  (:`Pressed`
    (`/Game/Blueprints/BP_BomberCharacter.SpawnBomb` (`self.Player1`))))

(event `InputAction|SpawnBomb2`
  (params (Key :type "Key Structure"))
  (:`Pressed`
    (`/Game/Blueprints/BP_BomberCharacter.SpawnBomb` (`self.Player2`))))

(fn `UserConstructionScript`)