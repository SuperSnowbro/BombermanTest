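; Game instance for a Bomber game that records round wins and presents the win screen.
; Its WinGame event adds a point to Player1Score or Player2Score for player index 0 or 1.
; It then creates UI_WinScreen, shows the first player controller's cursor, switches to UI-only input and sets the winner text from the raw zero-based index.
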(event `WinGame`
  (params (PlayerIndex :type Integer))
  (bind _returnvalue (`GameplayStatics.GetPlayerController` 0))
  (`|ExecutionSequence`
    (:`then_0`
      (switch `int` PlayerIndex
        (:`0`
          (`/Engine/EditorBlueprintResources/StandardMacros.IncrementInt` (`self.Player 1 score`)))
        (:`1`
          (`/Engine/EditorBlueprintResources/StandardMacros.IncrementInt` (`self.Player 2 score`)))))
    (:`then_1`
      (bind _returnvalue_2 (`|CreateWidget` "/Game/Blueprints/UserInterface/UI_WinScreen.UI_WinScreen_C"))
      (`UserWidget.AddToPlayerScreen` _returnvalue_2 0)
      (set `PlayerController.bShowMouseCursor` true _returnvalue)
      (`WidgetBlueprintLibrary.SetInputMode_UIOnlyEx` _returnvalue _returnvalue_2)
      (`/Game/Blueprints/UserInterface/UI_WinScreen.ChangeWinScreenText` _returnvalue_2 (`KismetTextLibrary.Conv_StringToText` (`KismetStringLibrary.Concat_StrStr` "Player " (`KismetStringLibrary.Conv_IntToString` PlayerIndex) " wins!"))))))