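; Bomb-spawning component that places regular bombs on behalf of its owning character.
; RequestBombSpawn checks the owner's bomb ammo, then spawns a BP_RegularBomb snapped to a grid at the character's position and a fixed height.
; The bomb receives the owner's detonation time, range and a player reference.
; A successful spawn decrements ammo, which the bomb is expected to restore when it explodes, per a graph comment.
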(fn `RequestBombSpawn`
  (returns (BombSpawned :type Boolean))
  (bind _myownercharacter (`self.MyOwnerCharacter`))
  (bind (_returnvalue_x _returnvalue_y) (`KismetMathLibrary.BreakVector` (`Actor.K2_GetActorLocation` (`self.MyOwnerCharacter`))))
  (if (> (`/Game/Blueprints/PlayerElements/BP_BomberCharacter.CurrentBombAmmo` (`self.MyOwnerCharacter`)) 0)
    (bind _returnvalue (`|SpawnActorFromClass` "/Game/Blueprints/Bombs/BP_RegularBomb.BP_RegularBomb_C" (`KismetMathLibrary.MakeTransform` (`KismetMathLibrary.MakeVector` (`KismetMathLibrary.Conv_IntToDouble` (`self.ConstrainPointToGrid` _returnvalue_x 50)) (`KismetMathLibrary.Conv_IntToDouble` (`self.ConstrainPointToGrid` _returnvalue_y 50)) 50.0)) "AlwaysSpawn" "OverrideRootScale" null (`/Game/Blueprints/PlayerElements/BP_BomberCharacter.BombDetonationTime` _myownercharacter) (`/Game/Blueprints/PlayerElements/BP_BomberCharacter.BombRange` _myownercharacter) (`self.MyOwnerCharacter`) null))
    (`/Engine/EditorBlueprintResources/StandardMacros.IsValid` _returnvalue ; check if we were not able to spawn the bomb for whatever reason
      (:`Is Valid`
        (`/Engine/EditorBlueprintResources/StandardMacros.DecrementInt` (`/Game/Blueprints/PlayerElements/BP_BomberCharacter.CurrentBombAmmo` (`self.MyOwnerCharacter`)) ; the bomb will get back at the player when it explodes and increment his bomb count
          (:`  `
            (return true))))
      (:`Is Not Valid`
        (return false)))))