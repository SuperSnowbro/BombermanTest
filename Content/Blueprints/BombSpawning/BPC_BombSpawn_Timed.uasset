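; Bomb-spawning component for timed bombs that lets its owning character place a BP_TimeBomb and detonate it on the next request.
; RequestBombSpawn spawns the bomb at the character's grid-snapped position with their BombRange, storing it and returning true on success.
; A DetonationSwitch flag makes the following request explode that bomb and clear the reference instead of spawning another.
; The Dismiss event explodes any bomb that is still valid.
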(event `self.Dismiss`
  (bind _currenttimebomb (`self.CurrentTimeBomb`))
  (`/Engine/EditorBlueprintResources/StandardMacros.IsValid` _currenttimebomb
    (:`Is Valid`
      (`/Game/Blueprints/Bombs/BP_TimeBomb.Explode` _currenttimebomb))))

(fn `RequestBombSpawn`
  (returns (BombSpawned :type Boolean))
  (bind (_returnvalue_x _returnvalue_y) (`KismetMathLibrary.BreakVector` (`Actor.K2_GetActorLocation` (`self.MyOwnerCharacter`))))
  (if (`self.DetonationSwitch`)
    (set `self.DetonationSwitch` false)
    (`/Game/Blueprints/Bombs/BP_TimeBomb.Explode` (`self.CurrentTimeBomb`))
    (set `self.CurrentTimeBomb` null) ; nullify reference after bomb detonation
    (else
      (bind _returnvalue (`|SpawnActorFromClass` "/Game/Blueprints/Bombs/BP_TimeBomb.BP_TimeBomb_C" (`KismetMathLibrary.MakeTransform` (`KismetMathLibrary.MakeVector` (`KismetMathLibrary.Conv_IntToDouble` (`self.ConstrainPointToGrid` _returnvalue_x 50)) (`KismetMathLibrary.Conv_IntToDouble` (`self.ConstrainPointToGrid` _returnvalue_y 50)) 50.0)) "AlwaysSpawn" "OverrideRootScale" null (`/Game/Blueprints/PlayerElements/BP_BomberCharacter.BombRange` (`self.MyOwnerCharacter`)) (`self.MyOwnerCharacter`) null))
      (`/Engine/EditorBlueprintResources/StandardMacros.IsValid` _returnvalue ; check if we were not able to spawn the bomb for whatever reason
        (:`Is Valid`
          (set `self.CurrentTimeBomb` _returnvalue)
          (set `self.DetonationSwitch` true)
          (return true))
        (:`Is Not Valid`
          (return false))))))